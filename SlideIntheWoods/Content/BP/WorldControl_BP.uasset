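; World controller Blueprint that changes atmosphere and progression according to the loop number stored in the GM_Ins game instance.
; The 检查 event maps certain loops to dimming the directional light with new ambience, flashlight and newspaper events (both empty stubs), or hidden level streaming.
; SetBGAudio fades between sounds on one audio component.
; The stored 音效 lets the temporary sliding sound revert to the current ambience when sliding ends.
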(event `self.ReceiveBeginPlay`
  (bind _nowaudio (`self.SetBGAudio` 1.0 "/Game/Audio/Background/default_forest_sounds.default_forest_sounds" 1.0))
  (set `self.音效` _nowaudio))

(event `检查`
  (bind _loopnumber (`/Game/BP/GM_Ins.LoopNumber` (cast `/Game/BP/GM_Ins` (`GameplayStatics.GetGameInstance`) :!pure true)))
  (`KismetSystemLibrary.PrintString` (`KismetStringLibrary.Concat_StrStr` "Loop Number:" (`KismetStringLibrary.Conv_IntToString` _loopnumber)))
  (switch `int` _loopnumber
    (:`3`
      (`self.天变昏暗`))
    (:`4`
      (`self.天黑`))
    (:`5`
      (`self.手电筒出现`))
    (:`6`
      (`self.报纸出现`))
    (:`9`
      (`self.关卡流送`))))

(event `天变昏暗`
  (`self.Change Light` 0)
  (bind _nowaudio (`self.SetBGAudio` 1.0 "/Game/Audio/Background/cave.cave" 1.0))
  (set `self.音效` _nowaudio))

(event `天黑`
  (`self.Change Light` 1)
  (bind _nowaudio (`self.SetBGAudio` 1.0 "/Game/Audio/Background/Nature_hoor.Nature_hoor" 1.0))
  (set `self.音效` _nowaudio))

(event `手电筒出现`)

(event `报纸出现`)

(event `敲打音`)

(event `尸体演出`)

(event `关卡流送`
  (`GameplayStatics.LoadStreamLevelBySoftObjectPtr` null))

(event `滑行`
  (`self.SetBGAudio` 1.0 "/Game/Audio/Sound/Effects/Huaxing.Huaxing" 1.0))

(event `结束滑行`
  (`self.SetBGAudio` 1.0 (`self.音效`) 1.0))

(fn `Change Light`
  (params (NewParam :type Integer))
  (switch `int` NewParam
    (:`0`
      (bind _returnvalue (`GameplayStatics.GetActorOfClass` "/Script/Engine.DirectionalLight"))
      (`LightComponent.SetIntensity` (`Light.LightComponent` _returnvalue) 2.0))
    (:`1`
      (bind _returnvalue_2 (`GameplayStatics.GetActorOfClass` "/Script/Engine.DirectionalLight"))
      (`LightComponent.SetIntensity` (`Light.LightComponent` _returnvalue_2) 0.15))))

(fn `UserConstructionScript`)